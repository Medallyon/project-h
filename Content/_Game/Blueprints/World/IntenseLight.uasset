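; IntenseLight is an end-of-game light that grows brighter and fades the screen as the player approaches.
; While active, Tick maps player distance to MaxIntensity and to the background opacity of the PH_Intros widget, both rising with proximity.
; When the player character overlaps its Collider, it calls EndOfGameReached.
; Construction assigns its PointLight to the Light variable, and BeginPlay caches the player and fade widget.
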(event OnComponentBeginOverlap(Collider)
  (params (OverlappedComponent :type Primitive%20Component%20Object%20Reference) (OtherActor :type Actor%20Object%20Reference) (OtherComp :type Primitive%20Component%20Object%20Reference) (OtherBodyIndex :type Integer) (bFromSweep :type Boolean) (SweepResult :type Hit%20Result%20Structure%20%28by%20ref%29))
  (if (Variables|Default|GetActive)
    (Utilities|Casting|CastToPH_Character_Default OtherActor)
    (Default|CallEndOfGameReached)))

(event EventBeginPlay
  (|CallParentFunction)
  (Utilities|FlowControl|Sequence
    (:then_0
      (bind _asph_character_default (Utilities|Casting|CastToPH_Character_Default (Pawn|GetControlledPawn (Game|GetPlayerController 0))))
      (Variables|Default|SetPlayer _asph_character_default))
    (:then_1
      (bind _foundwidgets (Widget|GetAllWidgetsOfClass "/Game/_Game/Blueprints/HUD/PH_Intros.PH_Intros_C" true))
      (Variables|Default|SetFade (Utilities|Array|Get(acopy) _foundwidgets)))))

(event EventTick
  (params (DeltaSeconds :type Float%20%28single-precision%29))
  (|CallParentFunction DeltaSeconds)
  (if (Variables|Default|GetActive)
    (bind _player (Variables|Default|GetPlayer)
      (:then
        (Variables|Default|SetMax%20Intensity (Math|Float|MapRangeClamped (Math|Vector|Distance(Vector) (Transformation|GetActorLocation) (Transformation|GetActorLocation _player)) 1e+04 5e+01 1e+05 1e+07))
        (bind _fade (Variables|Default|GetFade)
          (:then
            (Default|SetBackgroundOpacity _fade (Math|Float|MapRangeClamped (Math|Vector|Distance(Vector) (Transformation|GetActorLocation) (Transformation|GetActorLocation _player)) 6e+03 8e+02 0.0 1.0)))
          (:else)))
      (:else))))

(fn ConstructionScript
  (Variables|Default|SetLight (Variables|Default|GetPointLight))
  (|CallParentFunction))