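; Objective marker that changes the crazy-animal audio and opens up the next objectives when it advances the story.
; On AdvanceStoryImmediately it runs the parent logic, then sets a fixed volume multiplier on the audio component of every AS_CrazyAnimal actor.
; It then finds all ObjectiveMarkers, unlocks those with two hardcoded indices, and deactivates itself.
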(event EventAdvanceStoryImmediately
  (|CallParentFunction)
  (Utilities|FlowControl|Sequence
    (:then_0
      (bind _outactors (Actor|GetAllActorsOfClass "/Game/_Game/Blueprints/World/AS_CrazyAnimal.AS_CrazyAnimal_C"))
      (bind _arrayelement (Utilities|Array|ReverseforEachLoop _outactors)
        (:LoopBody
          (Audio|Components|Audio|SetVolumeMultiplier (Variables|/Script/Engine.AmbientSound|GetAudioComponent _arrayelement) 0.2 :!class /Script/Engine.AudioComponent))))
    (:then_1
      (bind _outactors_2 (Actor|GetAllActorsOfClass "/Game/_Game/Blueprints/World/ObjectiveMarker.ObjectiveMarker_C"))
      (bind _arrayelement_2 (Utilities|Array|ReverseforEachLoop _outactors_2)
        (:LoopBody
          (if (or (== (Variables|/Game/_Game/Blueprints/World/ObjectiveMarker.ObjectiveMarker_C|GetIndex _arrayelement_2) 5) (== (Variables|/Game/_Game/Blueprints/World/ObjectiveMarker.ObjectiveMarker_C|GetIndex _arrayelement_2) 6))
            (Variables|/Game/_Game/Blueprints/World/ObjectiveMarker.ObjectiveMarker_C|SetLocked _arrayelement_2 false)))))
    (:then_2
      (CallFunction|Deactivate))))

(fn ConstructionScript
  (|CallParentFunction))