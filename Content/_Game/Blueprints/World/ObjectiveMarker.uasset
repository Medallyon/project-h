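; World objective marker that guides the player with a bobbing visual and sound, then broadcasts ObjectiveFound with its index on reach.
; Activation unlocks and reveals it, fading audio in; Tick yaws it toward the player and raises pitch with proximity.
; Player overlap with the configurable sphere reports even while inactive unless locked; active markers play an audio/offset timeline, then deactivate.
; AdvanceStoryImmediately broadcasts without overlap; Overlapped is an empty hook.
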(event OnComponentBeginOverlap(Collision)
  (params (OverlappedComponent :type Primitive%20Component%20Object%20Reference) (OtherActor :type Actor%20Object%20Reference) (OtherComp :type Primitive%20Component%20Object%20Reference) (OtherBodyIndex :type Integer) (bFromSweep :type Boolean) (SweepResult :type Hit%20Result%20Structure%20%28by%20ref%29))
  (if (and (not (Variables|Default|GetObjective%20Overlapped)) (not (Variables|Default|GetLocked)))
    (Utilities|Casting|CastToPH_Character_Default OtherActor)
    (Utilities|FlowControl|Sequence
      (:then_0
        (Variables|Default|SetObjective%20Overlapped true)
        (CallFunction|Overlapped)
        (Default|CallObjectiveFound (Variables|Default|GetIndex)))
      (:then_1
        (if (Variables|Default|GetActive?)
          (bind (_direction _pitch _volume _z_offset) (Timeline|OnOverlap Play)
            (:Update
              (Utilities|FlowControl|Sequence
                (:then_0
                  (Audio|Components|Audio|SetPitchMultiplier (Variables|Components|GetAudioComponent) _pitch))
                (:then_1
                  (Audio|Components|Audio|SetVolumeMultiplier (Variables|Components|GetAudioComponent) _volume :!class /Script/Engine.AudioComponent))
                (:then_2
                  (Utilities|AddRelativeZLocation _z_offset false))))
            (:Finished
              (CallFunction|Deactivate))))))))

(event Custom|Float%20in%20world
  (params (Up? :type Boolean))
  (if Up?
    (bind _z_offset (Timeline|Float Play)
      (:Update
        (if (Variables|Default|GetObjective%20Overlapped)
          (Timeline|Float Stop)
          (else
            (Utilities|AddRelativeZLocation (* _z_offset (Variables|Default|GetMarker%20Float%20Max)) true))))
      (:Finished
        (if (not (Variables|Default|GetObjective%20Overlapped))
          (CallFunction|FloatinWorld (not Up?)))))
    (else
      (Timeline|Float Reverse))))

(event Custom|Activate
  (if (not (Variables|Default|GetObjective%20Overlapped))
    (Utilities|FlowControl|Sequence
      (:then_0
        (Variables|Default|SetActive? true)
        (Actor|Tick|SetActorTickEnabled true)
        (Variables|Default|SetLocked false)
        (Rendering|SetActorHiddenInGame false))
      (:then_1
        (bind _volume (Timeline|Increase%20Volume PlayFromStart)
          (:Update
            (Audio|Components|Audio|SetVolumeMultiplier (Variables|Components|GetAudioComponent) _volume :!class /Script/Engine.AudioComponent))))
      (:then_2
        (Variables|Default|SetWorld%20Origin (Transformation|GetActorLocation)))
      (:then_3
        (CallFunction|FloatinWorld true)))))

(event Custom|Deactivate
  (Utilities|FlowControl|Sequence
    (:then_0
      (Variables|Default|SetActive? false)
      (Rendering|SetActorHiddenInGame true))
    (:then_1
      (Audio|Components|Audio|SetVolumeMultiplier (Variables|Components|GetAudioComponent) 0.0 :!class /Script/Engine.AudioComponent))))

(event Custom|Advance%20Story%20Immediately
  (Default|CallObjectiveFound (Variables|Default|GetIndex)))

(event Custom|Overlapped)

(event EventTick
  (params (DeltaSeconds :type Float%20%28single-precision%29))
  (bind _returnvalue (Transformation|GetActorRotation))
  (if (Variables|Default|GetActive?)
    (Utilities|FlowControl|Sequence
      (:then_0
        (bind _player (Variables|Default|GetPlayer)
          (:then
            (Transformation|SetActorRotation (Math|Rotator|MakeRotator (.roll _returnvalue) (.pitch _returnvalue) (.yaw (Math|Rotator|FindLookatRotation (Transformation|GetActorLocation) (Transformation|GetActorLocation _player))))))
          (:else)))
      (:then_1
        (Audio|Components|Audio|SetPitchMultiplier (Variables|Components|GetAudioComponent) (Math|Float|MapRangeClamped (Math|Vector|Distance(Vector) (Transformation|GetActorLocation) (Transformation|GetActorLocation (Variables|Default|GetPlayer))) 1e+04 1e+03 1.0 2.0))))))

(event EventBeginPlay
  (Utilities|FlowControl|Sequence
    (:then_0
      (bind _outactors (Actor|GetAllActorsOfClass "/Game/_Game/Blueprints/Character/PH_Character_Default.PH_Character_Default_C"))
      (Variables|Default|SetPlayer (Utilities|Array|Get(acopy) _outactors)))
    (:then_1
      (if (not (Variables|Default|GetActive?))
        (CallFunction|Deactivate)))))

(fn ConstructionScript
  (Utilities|FlowControl|Sequence
    (:then_0
      (Components|Sphere|SetSphereRadius (Variables|Default|GetCollision) (Variables|Default|GetPlayer%20Detection) true))
    (:then_1
      (Transformation|AddRelativeLocation (Variables|Default|GetCollision) (Variables|Default|GetDetection%20Radius%20Offset) false false))))