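; Fireplace world actor with fire, smoke and light components that can be shown lit or unlit.
; The construction script drives component visibility from two flags: Enabled controls Fire and Smoke, while Light requires both UseLight and Enabled.
; An earlier Light visibility call based on UseLight alone is overridden later in the same sequence.
; The event graph holds only disabled placeholder events, so it adds no runtime behavior.
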(event EventBeginPlay)

(event Collision|EventActorBeginOverlap
  (params (OtherActor :type Actor%20Object%20Reference)))

(event EventTick
  (params (DeltaSeconds :type Float%20%28single-precision%29)))

(fn ConstructionScript
  (Utilities|FlowControl|Sequence
    (:then_0
      (Rendering|SetVisibility (Variables|Default|GetLight) (Variables|Default|GetUse%20Light) false))
    (:then_1
      (Rendering|SetVisibility (Variables|Default|GetFire) (Variables|Default|GetEnabled) false)
      (Rendering|SetVisibility (Variables|Default|GetSmoke) (Variables|Default|GetEnabled) false)
      (Rendering|SetVisibility (Variables|Default|GetLight) (and (Variables|Default|GetUse%20Light) (Variables|Default|GetEnabled)) false))))