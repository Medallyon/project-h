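; LakeWaterPlane is a configurable lake water surface whose look is set up in the construction script.
; InitialWaterCreation creates a dynamic material instance from OceanMaterial on the WaterSurface component and scales that component in X and Y.
; The construction script then pushes the water scale, variation, wave speed and two color variables into that material instance as parameters.
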(fn ConstructionScript
  (|InitialWaterCreation)
  (Rendering|Material|SetScalarParameterValue (Variables|Default|GetWater%20Material) "Water Scale" (Variables|Default|GetOverall%20Water%20Scale) :!class /Script/Engine.MaterialInstanceDynamic)
  (Rendering|Material|SetScalarParameterValue (Variables|Default|GetWater%20Material) "Variation Amount" (Variables|Default|GetVariation%20Amount) :!class /Script/Engine.MaterialInstanceDynamic)
  (Rendering|Material|SetScalarParameterValue (Variables|Default|GetWater%20Material) "Wave Speed" (Variables|Default|GetWave%20Speed) :!class /Script/Engine.MaterialInstanceDynamic)
  (Rendering|Material|SetVectorParameterValue (Variables|Default|GetWater%20Material) "WaterColor A" (Variables|Default|GetPrimary%20Water%20Color) :!class /Script/Engine.MaterialInstanceDynamic)
  (Rendering|Material|SetVectorParameterValue (Variables|Default|GetWater%20Material) "WaterColor B" (Variables|Default|GetSecondary%20Water%20Color) :!class /Script/Engine.MaterialInstanceDynamic))