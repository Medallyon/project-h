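; InspectableClue is a world object carrying a clue that can be found, with an optional action triggered on discovery.
; The construction script applies configurable meshes to the object and clue, scales the clue and its trigger box, and offsets both.
; ClueFound extends the parent's logic: if UseOnFind is set and the added item has a valid UseAction class, it schedules that actor's delayed spawn and immediately opens the referenced Door.
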(fn ConstructionScript
  (bind _clue (Variables|Default|GetClue))
  (|CallParentFunction)
  (Utilities|FlowControl|Sequence
    (:then_0
      (bind _object_mesh (Variables|InspectionSetup|GetObject%20Mesh)
        (:then
          (Components|StaticMesh|SetStaticMesh (Variables|Default|GetObject) _object_mesh))
        (:else)))
    (:then_1
      (Utilities|FlowControl|Sequence
        (:then_0
          (bind _clue_mesh (Variables|InspectionSetup|Clue|GetClue%20Mesh)
            (:then
              (Components|StaticMesh|SetStaticMesh (Variables|Default|GetClue) _clue_mesh)
              (Transformation|SetRelativeScale3D _clue (* (Variables|/Script/Engine.SceneComponent|GetRelativeScale3D _clue) (Variables|InspectionSetup|Clue|GetClue%20Scale)))
              (Components|Box|SetBoxExtent (Variables|Default|GetClueTrigger) (Variables|InspectionSetup|Clue|GetClue%20Trigger%20Scale) true))
            (:else)))
        (:then_1
          (Transformation|AddRelativeLocation (Variables|Default|GetClue) (Variables|InspectionSetup|Clue|GetClue%20Offset) false false)
          (Transformation|AddRelativeLocation (Variables|Default|GetClueTrigger) (Variables|InspectionSetup|Clue|GetClue%20Trigger%20Offset) false false))))))

(fn ClueFound
  (bind _addeditem (Variables|Default|GetAddedItem))
  (|CallParentFunction)
  (if (Variables|Default|GetUse%20on%20Find)
    (if (Utilities|IsValidClass (.useaction _addeditem))
      (Variables|Default|SetUse%20Action (.useaction _addeditem))
      (Utilities|Time|SetTimerbyFunctionName 0 "Use Item" (Variables|Default|GetUse%20Action%20Delay))
      (Default|OpenDoor (Variables|Default|GetDoor)))))

(fn UseItem
  (Game|SpawnActorfromClass (Variables|Default|GetUse%20Action) (Math|Transform|MakeTransform "0, 0, 0" "0, 0, 0" "1,1,1") "Undefined" 0 0 0))